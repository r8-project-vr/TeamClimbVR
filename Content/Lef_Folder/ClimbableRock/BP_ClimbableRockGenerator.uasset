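; BP_ClimbableRockGenerator is a generator that spawns climbable rocks at varying heights for the VR climbing pawn.
; BeginPlay caches the player's VRPawn_Climb as CharacterRef.
; SpawnNextClimbableRock spawns RockClass at a random horizontal X offset from the player and a random vertical gap above HighestGeneratedZ, leaving Y unset.
; The file neither calls this function nor updates HighestGeneratedZ.
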(event EventBeginPlay
  (bind _asvrpawn_climb (Utilities|Casting|CastToVRPawn_Climb (Game|Player|GetPlayerPawn 0)))
  (Variables|Default|SetCharacterRef _asvrpawn_climb))

(event Collision|EventActorBeginOverlap
  (params (OtherActor :type Actor%20Object%20Reference)))

(event EventTick
  (params (DeltaSeconds :type Float%20%28single-precision%29)))

(fn ConstructionScript)

(fn SpawnNextClimbableRock
  (Game|SpawnActorfromClass (Variables|Default|GetRockClass) (Math|Transform|MakeTransform (Math|Vector|MakeVector (+ (.x (Transformation|GetActorLocation (Variables|Default|GetCharacterRef))) (Math|Random|RandomFloatinRange (* (Variables|Default|GetMaxHorizontalSpread) -1.0) (Variables|Default|GetMaxHorizontalSpread))) 0.0 (+ (Variables|Default|GetHighestGeneratedZ) (Math|Random|RandomFloatinRange (Variables|Default|GetMinVerticalGap) (Variables|Default|GetMaxVerticalGap)))) "0, 0, 0" "1.000000,1.000000,1.000000") "Undefined" "MultiplyWithRoot" 0 0))