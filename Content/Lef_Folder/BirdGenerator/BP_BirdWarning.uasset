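; BP_BirdWarning is a short-lived warning marker actor, apparently signalling an incoming bird in the bird generator system.
; On BeginPlay, the WarningPulse timeline drives the uniform world scale of BirdWarningWidget to make it pulse, and the actor destroys itself after a fixed delay.
; Every tick it rotates to face the player camera, acting as a billboard.
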(event EventBeginPlay
  (Utilities|FlowControl|Sequence
    (:then_0
      (bind _scale (Timeline|WarningPulse PlayFromStart)
        (:Update
          (Transformation|SetWorldScale3D (Variables|Default|GetBirdWarningWidget) (Math|Vector|MakeVector _scale _scale _scale)))))
    (:then_1
      (Utilities|FlowControl|Delay 5.0)
      (Actor|DestroyActor))))

(event Collision|EventActorBeginOverlap
  (params (OtherActor :type Actor%20Object%20Reference)))

(event EventTick
  (params (DeltaSeconds :type Float%20%28single-precision%29))
  (Transformation|SetActorRotation (Math|Rotator|FindLookatRotation (Transformation|GetActorLocation) (Camera|GetCameraLocation (Game|GetPlayerCameraManager 0)))))

(fn ConstructionScript)