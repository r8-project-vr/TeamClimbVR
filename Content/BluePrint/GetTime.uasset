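; GetTime is a timer Blueprint that triggers a teleport once a time limit is exceeded.
; While IsCount is set, Tick adds world delta seconds to Time.
; When Time passes TimeLimit, it looks up a TeleportTrigger actor by class and calls TriggerTeleport.
; Time and IsCount are not reset here, so the call repeats every tick while counting stays on.
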(event EventBeginPlay)

(event Collision|EventActorBeginOverlap
  (params (OtherActor :type Actor%20Object%20Reference)))

(event EventTick
  (params (DeltaSeconds :type Float%20%28single-precision%29))
  (if (Variables|Default|GetisCount)
    (Variables|Default|SetTime (+ (Variables|Default|GetTime) (Utilities|Time|GetWorldDeltaSeconds)))
    (if (> (Variables|Default|GetTime) (Variables|Default|GetTimeLimit))
      (bind _returnvalue (Actor|GetActorOfClass "/Script/TeamClimbVR.ATeleportTrigger"))
      (Class|ATeleportTrigger|TriggerTeleport _returnvalue))))

(fn ConstructionScript)