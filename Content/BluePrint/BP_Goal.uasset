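; BP_Goal is the goal actor that runs the level-clear sequence when its OnPlayerReachedGoal event fires.
; The event shows its Widget, plays a stadium cheer, calls GameCleared on the GameResultManager and stops counting on every GetTime actor.
; After a short delay it opens the level named by LevelName.
; Its own overlap event is unused, so this graph does not detect the player itself.
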(event EventBeginPlay)

(event Collision|EventActorBeginOverlap
  (params (OtherActor :type Actor%20Object%20Reference)))

(event EventTick
  (params (DeltaSeconds :type Float%20%28single-precision%29)))

(event EventOnPlayerReachedGoal
  (Rendering|SetVisibility (Variables|Default|GetWidget) true false)
  (bind _returnvalue (Actor|GetActorOfClass "/Script/TeamClimbVR.GameResultManager"))
  (Audio|PlaySoundatLocation "/Game/BGM_SE/スタジアムの歓声1_Cue.スタジアムの歓声1_Cue" "0, 0, 0" "0, 0, 0" 1.0 1.0 0.0 0 0 0 0)
  (Class|GameResultManager|GameCleared _returnvalue)
  (bind _outactors (Actor|GetAllActorsOfClass "/Game/BluePrint/GetTime.GetTime_C"))
  (for _array_element _outactors
    (Variables|/Game/BluePrint/GetTime.GetTime_C|SetisCount _array_element false))
  (Utilities|FlowControl|Delay 5.0)
  (Game|OpenLevel(byName) (Variables|Default|GetLevelName)))

(fn ConstructionScript)