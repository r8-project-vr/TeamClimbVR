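; DayCycleLight1 is a day cycle light Blueprint that turns from its starting rotation to a target direction over a time limit.
; BeginPlay stores the current world rotation as the start.
; Each Tick accumulates delta time and sets the world rotation with a shortest-path rotator lerp, using elapsed time over the limit as the clamped alpha.
; The rotation runs one way and holds at the target, with no looping.
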(event EventBeginPlay
  (Variables|Default|SetstartDir (Transformation|GetWorldRotation)))

(event EventTick
  (params (DeltaSeconds :type Float%20%28single-precision%29))
  (Variables|Default|SetSecond (+ (Variables|Default|GetSecond) (Utilities|Time|GetWorldDeltaSeconds)))
  (Transformation|SetWorldRotation (Math|Rotator|Lerp(Rotator) (Variables|Default|GetstartDir) (Variables|Default|GettargetDir) (Math|Float|Clamp(Float) (Math|Float|SafeDivide (Variables|Default|GetSecond) (Variables|Default|GetTimeLimit))) true) false false))